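; Stealth system pickup actor that adds a throwable item, either a rock or a smoke bomb, to the interacting actor's inventory.
; The construction script sets the Sphere component's static mesh to match the selected Type.
; On Interact, it passes the Type to the actor's StealthComponent and destroys itself, doing nothing if that component is absent.
; Its interaction functions never block interaction and return no custom text.
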(event `/Game/StealthSystem/Player/Interfaces/BPI_Interaction.Interact`
  (params (Actor :type "Actor Object Reference"))
  (bind _returnvalue (`self.GetComponentByClass` Actor "/Game/StealthSystem/Player/Components/StealthComponent.StealthComponent_C"))
  ;[0.1094 0.1094 0.1094] This logic adds the item to the player inventory upon overlap.
  (`/Engine/EditorBlueprintResources/StandardMacros.IsValid` _returnvalue
    (:`Is Valid`
      (`/Game/StealthSystem/Player/Components/StealthComponent.AddInventoryItem` _returnvalue (`self.Type`))
      (`self.K2_DestroyActor`))))

(fn `InteractionBlocked`
  (returns (Result :type Boolean))
  (return false))

(fn `InteractionCustomText`
  (returns (Text :type Text))
  (return ""))

(fn `UserConstructionScript`
  (switch `/Game/StealthSystem/Pickups/Enum_InventoryType` (`self.Type`)
    (:`NewEnumerator0`
      (`StaticMeshComponent.SetStaticMesh` (`self.Sphere`) "/Game/StealthSystem/Pickups/Pickup_Rock.Pickup_Rock"))
    (:`NewEnumerator1`
      (`StaticMeshComponent.SetStaticMesh` (`self.Sphere`) "/Game/StealthSystem/Pickups/Pickup_SmokeBomb.Pickup_SmokeBomb"))))